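; Large left door actor that swings open and closed in response to OnOpen and OnClose events from its OpenDoor component.
; It caches its starting rotation on BeginPlay.
; A timeline, played on open and reversed on close, interpolates yaw from zero to OpenYaw and combines it with that cached rotation to rotate the whole actor.
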(event OnOpen(OpenDoor)
  (bind _doorrotation (Timeline|OpenDoorTimeline Play)
    (:Update
      (Transformation|SetActorRotation (Math|Rotator|CombineRotators (Math|Rotator|MakeRotator 0.0 0.0 (Math|Float|Lerp 0.0 (Variables|Default|GetOpenYaw) _doorrotation)) (Variables|Default|GetInitialRotation))))))

(event OnClose(OpenDoor)
  (bind _doorrotation (Timeline|OpenDoorTimeline Reverse)
    (:Update
      (Transformation|SetActorRotation (Math|Rotator|CombineRotators (Math|Rotator|MakeRotator 0.0 0.0 (Math|Float|Lerp 0.0 (Variables|Default|GetOpenYaw) _doorrotation)) (Variables|Default|GetInitialRotation))))))

(event EventBeginPlay
  (Variables|Default|SetInitialRotation (Transformation|GetActorRotation)))

(event Collision|EventActorBeginOverlap
  (params (OtherActor :type Actor%20Object%20Reference)))

(event EventTick
  (params (DeltaSeconds :type Float%20%28single-precision%29)))

(fn ConstructionScript)